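; BP_MBFPSMainHUD is the first-person shooter HUD Blueprint that creates and manages the main HUD and in-game menu widgets.
; Custom events add both widgets to the viewport, with the menu starting hidden.
; Toggling the menu flips its visibility, mouse cursor and input mode, centering the cursor when it opens.
; Damage feedback plays a timeline that feeds its alpha into the main HUD widget each update.
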(event Custom|CenterMouse
  (params (PlayerController :type Player%20Controller%20Object%20Reference))
  (bind _returnvalue (Viewport|GetViewportSize))
  ;[0.2564 1 0.8598] Center Mouse Cursor
  (Class|PlayerController|SetMouseLocation PlayerController (Math|Float|Truncate (/ (.x _returnvalue) 2.0)) (Math|Float|Truncate (/ (.y _returnvalue) 2.0))))

(event Custom|ClientDamageFeedback
  ;[1 1 1] Damage Feedback
  (bind _alpha (Timeline|DamageFeecbackTimeLine PlayFromStart)
    (:Update
      (Default|DamageFeedback (Variables|Default|GetMainHUD) _alpha))))

(event EventToggleinGameMenu
  (bind _returnvalue (Game|Player|GetOwningPlayerController))
  (bind _returnvalue_2 (Game|Player|GetOwningPlayerController))
  ;[0.237 0.8191 1] Toggle In game menu
  (if (Variables|Default|GetbInGameMenuActive)
    (Variables|Default|SetbInGameMenuActive false)
    (Widget|SetVisibility (Variables|Default|GetinGameMenu) "Hidden")
    (Variables|/Script/Engine.PlayerController|SetbShowMouseCursor _returnvalue_2 false)
    (Input|SetInputModeGameOnly _returnvalue_2)
    (else
      (Variables|Default|SetbInGameMenuActive true)
      (Widget|SetVisibility (Variables|Default|GetinGameMenu) "Visible")
      (Variables|/Script/Engine.PlayerController|SetbShowMouseCursor _returnvalue true)
      (Input|SetInputModeUIOnly _returnvalue (Variables|Default|GetinGameMenu) "DoNotLock")
      (CallFunction|CenterMouse _returnvalue))))

(event EventCreateinGameMenu
  ;[0.3229 1 0.4004] Create In game menu
  (bind _returnvalue (UserInterface|CreateWidget "/Game/Widgets/Menu/WBP_InGameMenu.WBP_InGameMenu_C"))
  (bind _output_get (Variables|Default|SetinGameMenu _returnvalue))
  (UserInterface|Viewport|AddtoViewport _output_get 0)
  (Widget|SetVisibility _output_get "Hidden")
  (Variables|Default|SetbInGameMenuActive false))

(event EventDamageFeedback
  ;[1 1 1] Damage Feedback
  (CallFunction|ClientDamageFeedback))

(event EventCreateMainHUD
  ;[0.1946 0.9303 1] Create MainHUD
  (bind _returnvalue (UserInterface|CreateWidget "/Game/Widgets/PlayerHUD/WBP_MainHUD.WBP_MainHUD_C"))
  (bind _output_get (Variables|Default|SetMainHUD _returnvalue))
  (UserInterface|Viewport|AddtoViewport _output_get 0))

(fn ConstructionScript)