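; BP_FPSMBCharacter is the first-person shooter player character Blueprint that links the pawn to the main HUD.
; For the locally controlled player, it waits briefly on BeginPlay, then caches the MainHUD widget and sets up its health-changed binding.
; SetAimingCrosshair hides the crosshair while aiming, reaching it through the player controller's HUD.
; OnDeathHUD notifies the cached widget of death.
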(event EventBeginPlay
  ;[1 0.2272 0.1973] Bind OnHeathChanged Event on MainHUD
  (if (Pawn|IsLocallyControlled)
    (Utilities|FlowControl|Delay 0.1)
    (bind _asbp_fpsmbplayer_controller (Utilities|Casting|CastToBP_FPSMBPlayerController (Pawn|GetController)))
    (Utilities|IsValid (HUD|GetHUD _asbp_fpsmbplayer_controller)
      (:Is%20Valid
        (bind _asbp_mbfpsmain_hud (Utilities|Casting|CastToBP_MBFPSMainHUD (HUD|GetHUD _asbp_fpsmbplayer_controller)))
        (bind _output_get (Variables|Default|SetMain%20HUD (Variables|/Game/Blueprints/HUD/BP_MBFPSMainHUD.BP_MBFPSMainHUD_C|GetMainHUD _asbp_mbfpsmain_hud)))
        (Default|SetonHealthChanged _output_get)))))

(event EventOnDeathHUD
  (bind _main_hud (Variables|Default|GetMain%20HUD))
  ;[1 0.1036 0.1335] UnBind OnHealthChanged Event
  (Utilities|IsValid _main_hud
    (:Is%20Valid
      (Default|OnDeath _main_hud))))

(event EventSetAimingCrosshair
  (params (bIsAimVal :type Boolean))
  ;[1 0.995 0.155] Set Aiming to Crosshair
  (bind _asbp_fpsmbplayer_controller (Utilities|Casting|CastToBP_FPSMBPlayerController (Pawn|GetController)))
  (if (Pawn|IsLocallyControlled)
    (bind _returnvalue (Class|FPSMBPlayerController|GetMBFPSMainHUD _asbp_fpsmbplayer_controller))
    (bind _asbp_mbfpsmain_hud (Utilities|Casting|CastToBP_MBFPSMainHUD _returnvalue))
    (Default|SetCrosshairVisivility (Variables|/Game/Widgets/WBP_MainHUD.WBP_MainHUD_C|GetWBP_Crosshair (Variables|/Game/Blueprints/HUD/BP_MBFPSMainHUD.BP_MBFPSMainHUD_C|GetMainHUD _asbp_mbfpsmain_hud)) (not bIsAimVal))))

(fn ConstructionScript)