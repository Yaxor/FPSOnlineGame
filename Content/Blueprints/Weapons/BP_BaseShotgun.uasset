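; Base shotgun weapon Blueprint that drives camera recoil on the owning player's controller.
; WeaponRecoil saves the starting pitch once per recoil cycle, then plays a timeline that adds pitch and yaw input.
; When that timeline finishes, or StopWeaponRecoil interrupts it for the locally controlled character, a second timeline lerps pitch back to the saved value.
; The return handles pitch wraparound at 360 degrees and stops within an offset tolerance; yaw is not restored.
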(event EventWeaponRecoil
  (Variables|Default|SetbFire true)
  (Utilities|FlowControl|Sequence
    (:then_0
      (Utilities|FlowControl|DoOnce false :!label _label
        (:Completed
          ;[1 1 1] Set Initial Pitch
          (bind _myplayercontroller (CallFunction|GetMyPlayerController))
          (if (<= (.Pitch (Math|Rotator|BreakRotator (Pawn|GetControlRotation _myplayercontroller :!class /Script/Engine.Controller))) 9e+01)
            (Variables|Default|SetInitial%20Pitch (.Pitch (Math|Rotator|BreakRotator (Pawn|GetControlRotation _myplayercontroller :!class /Script/Engine.Controller))))
            (else
              (Variables|Default|SetInitial%20Pitch (- (.Pitch (Math|Rotator|BreakRotator (Pawn|GetControlRotation _myplayercontroller :!class /Script/Engine.Controller))) 3.6e+02)))))))
    (:then_1
      (bind (_direction _pitchinput _yawinput) (Timeline|RecoilTimeline PlayFromStart)
        (:Update
          (CallFunction|ApplyRecoil _pitchinput _yawinput))
        (:Finished
          (Variables|Default|SetbFinished true)
          (Utilities|FlowControl|Sequence
            (:then_0
              (Timeline|RecoilTimeline Stop))
            (:then_1
              (Components|Timeline|SetPlayRate (Variables|Default|GetStopRecoilTimeline) 1.0)
              (bind _alpha (Timeline|StopRecoilTimeline PlayFromStart)
                (:Update
                  ;[1 1 1] Return to center
                  (bind _myplayercontroller_2 (CallFunction|GetMyPlayerController))
                  (if (<= (.Pitch (Math|Rotator|BreakRotator (Pawn|GetControlRotation _myplayercontroller_2 :!class /Script/Engine.Controller))) 9e+01)
                    (Pawn|SetControlRotation _myplayercontroller_2 (Math|Rotator|MakeRotator (.Roll (Math|Rotator|BreakRotator (Pawn|GetControlRotation _myplayercontroller_2 :!class /Script/Engine.Controller))) (Math|Float|Lerp (.Pitch (Math|Rotator|BreakRotator (Pawn|GetControlRotation _myplayercontroller_2 :!class /Script/Engine.Controller))) (Variables|Default|GetInitial%20Pitch) _alpha) (.Yaw (Math|Rotator|BreakRotator (Pawn|GetControlRotation _myplayercontroller_2 :!class /Script/Engine.Controller)))))
                    (else
                      (Pawn|SetControlRotation _myplayercontroller_2 (Math|Rotator|MakeRotator (.Roll (Math|Rotator|BreakRotator (Pawn|GetControlRotation _myplayercontroller_2 :!class /Script/Engine.Controller))) (Math|Float|Lerp (- (.Pitch (Math|Rotator|BreakRotator (Pawn|GetControlRotation _myplayercontroller_2 :!class /Script/Engine.Controller))) 3.6e+02) (Variables|Default|GetInitial%20Pitch) _alpha) (.Yaw (Math|Rotator|BreakRotator (Pawn|GetControlRotation _myplayercontroller_2 :!class /Script/Engine.Controller)))))))
                  (bind _myplayercontroller_3 (CallFunction|GetMyPlayerController))
                  (if (<= (Math|Float|Absolute(Float) (- (.Pitch (Math|Rotator|BreakRotator (Pawn|GetControlRotation _myplayercontroller_3 :!class /Script/Engine.Controller))) (Variables|Default|GetInitial%20Pitch))) (Variables|Default|GetStopRecoilOffset))
                    (Variables|Default|SetInitial%20Pitch 0.0)
                    (Timeline|StopRecoilTimeline Stop)))))
            (:then_2
              (goto _label Reset))))))
    (:then_2
      (Timeline|StopRecoilTimeline Stop))))

(event EventStopWeaponRecoil
  (bind _asfpsmbcharacter (Utilities|Casting|CastToFPSMBCharacter (Components|GetOwner)))
  (if (Pawn|IsLocallyControlled _asfpsmbcharacter)
    (if (and (not (Variables|Default|GetbFinished)) (Variables|Default|GetbFire))
      (Variables|Default|SetbFire false)
      (Utilities|FlowControl|Sequence :!label _label
        (:then_0
          (bind (_direction _pitchinput _yawinput) (Timeline|RecoilTimeline Stop)
            (:Update
              (CallFunction|ApplyRecoil _pitchinput _yawinput))
            (:Finished
              (Variables|Default|SetbFinished true)
              (goto _label))))
        (:then_1
          (Components|Timeline|SetPlayRate (Variables|Default|GetStopRecoilTimeline) 1.0)
          (bind _alpha (Timeline|StopRecoilTimeline PlayFromStart)
            (:Update
              ;[1 1 1] Return to center
              (bind _myplayercontroller (CallFunction|GetMyPlayerController))
              (if (<= (.Pitch (Math|Rotator|BreakRotator (Pawn|GetControlRotation _myplayercontroller :!class /Script/Engine.Controller))) 9e+01)
                (Pawn|SetControlRotation _myplayercontroller (Math|Rotator|MakeRotator (.Roll (Math|Rotator|BreakRotator (Pawn|GetControlRotation _myplayercontroller :!class /Script/Engine.Controller))) (Math|Float|Lerp (.Pitch (Math|Rotator|BreakRotator (Pawn|GetControlRotation _myplayercontroller :!class /Script/Engine.Controller))) (Variables|Default|GetInitial%20Pitch) _alpha) (.Yaw (Math|Rotator|BreakRotator (Pawn|GetControlRotation _myplayercontroller :!class /Script/Engine.Controller)))))
                (else
                  (Pawn|SetControlRotation _myplayercontroller (Math|Rotator|MakeRotator (.Roll (Math|Rotator|BreakRotator (Pawn|GetControlRotation _myplayercontroller :!class /Script/Engine.Controller))) (Math|Float|Lerp (- (.Pitch (Math|Rotator|BreakRotator (Pawn|GetControlRotation _myplayercontroller :!class /Script/Engine.Controller))) 3.6e+02) (Variables|Default|GetInitial%20Pitch) _alpha) (.Yaw (Math|Rotator|BreakRotator (Pawn|GetControlRotation _myplayercontroller :!class /Script/Engine.Controller)))))))
              (bind _myplayercontroller_2 (CallFunction|GetMyPlayerController))
              (if (<= (Math|Float|Absolute(Float) (- (.Pitch (Math|Rotator|BreakRotator (Pawn|GetControlRotation _myplayercontroller_2 :!class /Script/Engine.Controller))) (Variables|Default|GetInitial%20Pitch))) (Variables|Default|GetStopRecoilOffset))
                (Variables|Default|SetInitial%20Pitch 0.0)
                (Timeline|StopRecoilTimeline Stop)))))
        (:then_2
          (Utilities|FlowControl|DoOnce false) ; enters at Reset
        )))))

(fn ConstructionScript)

(fn GetMyPlayerController
  (bind _aspawn (Utilities|Casting|CastToPawn (Components|GetOwner)))
  (bind _asplayer_controller (Utilities|Casting|CastToPlayerController (Pawn|GetController _aspawn)))
  (return _asplayer_controller))

(fn ApplyRecoil
  (params (PitchInput :type Float%20%28single-precision%29) (yawInput :type Float%20%28single-precision%29))
  (bind _myplayercontroller (CallFunction|GetMyPlayerController))
  (Class|PlayerController|AddPitchInput _myplayercontroller (* PitchInput -1.0))
  (Class|PlayerController|AddYawInput _myplayercontroller yawInput))