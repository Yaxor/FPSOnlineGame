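; Base AK47 weapon Blueprint that drives camera recoil and pushes ammo counts and the weapon icon to the owning player's HUD.
; WeaponRecoil saves the initial pitch once per burst, then plays a timeline that feeds pitch and yaw input to the controller.
; StopWeaponRecoil, for locally controlled owners, starts a second timeline that lerps pitch back to the saved value, stopping when close or when firing resumes.
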(event EventWeaponRecoil
  (Variables|Default|SetbFire true)
  (Utilities|FlowControl|Sequence
    (:then_0
      (Utilities|FlowControl|DoOnce false
        (:Completed
          ;[1 1 1] Set Initial Pitch
          (bind _myplayercontroller (CallFunction|GetMyPlayerController))
          (if (<= (.Pitch (Math|Rotator|BreakRotator (Pawn|GetControlRotation _myplayercontroller :!class /Script/Engine.Controller))) 9e+01)
            (Variables|Default|SetInitialPitch (.Pitch (Math|Rotator|BreakRotator (Pawn|GetControlRotation _myplayercontroller :!class /Script/Engine.Controller))))
            (else
              (Variables|Default|SetInitialPitch (- (.Pitch (Math|Rotator|BreakRotator (Pawn|GetControlRotation _myplayercontroller :!class /Script/Engine.Controller))) 3.6e+02)))))))
    (:then_1
      (if (Variables|Default|GetbFinished)
        (Variables|Default|SetbFinished false)
        (bind (_direction _pitchinput _yawinput) (Timeline|RecoilTimeline PlayFromStart)
          (:Update
            (CallFunction|ApplyRecoil _pitchinput _yawinput)
            (if (not (Variables|Default|GetbFire))
              (Variables|Default|SetbFinished true)
              (Timeline|RecoilTimeline Stop))))))
    (:then_2
      (bind _alpha (Timeline|StopRecoilTimeLine Stop)
        (:Update
          (if (Variables|Default|GetbFire)
            (Timeline|StopRecoilTimeLine Stop)
            (else
              ;[1 1 1] Return to center
              (bind _myplayercontroller_2 (CallFunction|GetMyPlayerController))
              (if (<= (.Pitch (Math|Rotator|BreakRotator (Pawn|GetControlRotation _myplayercontroller_2 :!class /Script/Engine.Controller))) 9e+01)
                (Pawn|SetControlRotation _myplayercontroller_2 (Math|Rotator|MakeRotator (.Roll (Math|Rotator|BreakRotator (Pawn|GetControlRotation _myplayercontroller_2 :!class /Script/Engine.Controller))) (Math|Float|Lerp (.Pitch (Math|Rotator|BreakRotator (Pawn|GetControlRotation _myplayercontroller_2 :!class /Script/Engine.Controller))) (Variables|Default|GetInitialPitch) _alpha) (.Yaw (Math|Rotator|BreakRotator (Pawn|GetControlRotation _myplayercontroller_2 :!class /Script/Engine.Controller)))))
                (else
                  (Pawn|SetControlRotation _myplayercontroller_2 (Math|Rotator|MakeRotator (.Roll (Math|Rotator|BreakRotator (Pawn|GetControlRotation _myplayercontroller_2 :!class /Script/Engine.Controller))) (Math|Float|Lerp (- (.Pitch (Math|Rotator|BreakRotator (Pawn|GetControlRotation _myplayercontroller_2 :!class /Script/Engine.Controller))) 3.6e+02) (Variables|Default|GetInitialPitch) _alpha) (.Yaw (Math|Rotator|BreakRotator (Pawn|GetControlRotation _myplayercontroller_2 :!class /Script/Engine.Controller)))))))
              (bind _myplayercontroller_3 (CallFunction|GetMyPlayerController))
              (if (<= (Math|Float|Absolute(Float) (- (.Pitch (Math|Rotator|BreakRotator (Pawn|GetControlRotation _myplayercontroller_3 :!class /Script/Engine.Controller))) (Variables|Default|GetInitialPitch))) 0.5)
                (Variables|Default|SetInitialPitch 0.0)
                (Timeline|StopRecoilTimeLine Stop)))))))))

(event EventStopWeaponRecoil
  (Utilities|FlowControl|Delay 0.05)
  (bind _asfpsmbcharacter (Utilities|Casting|CastToFPSMBCharacter (Components|GetOwner)))
  (if (Pawn|IsLocallyControlled _asfpsmbcharacter)
    (if (Variables|Default|GetbFire)
      (Variables|Default|SetbFire false)
      (Utilities|FlowControl|Sequence
        (:then_0
          (Utilities|FlowControl|DoOnce false) ; enters at Reset
        )
        (:then_1
          (Components|Timeline|SetPlayRate (Variables|Default|GetStopRecoilTimeLine) 1.5)
          (bind _alpha (Timeline|StopRecoilTimeLine PlayFromStart)
            (:Update
              (if (Variables|Default|GetbFire)
                (Timeline|StopRecoilTimeLine Stop)
                (else
                  ;[1 1 1] Return to center
                  (bind _myplayercontroller (CallFunction|GetMyPlayerController))
                  (if (<= (.Pitch (Math|Rotator|BreakRotator (Pawn|GetControlRotation _myplayercontroller :!class /Script/Engine.Controller))) 9e+01)
                    (Pawn|SetControlRotation _myplayercontroller (Math|Rotator|MakeRotator (.Roll (Math|Rotator|BreakRotator (Pawn|GetControlRotation _myplayercontroller :!class /Script/Engine.Controller))) (Math|Float|Lerp (.Pitch (Math|Rotator|BreakRotator (Pawn|GetControlRotation _myplayercontroller :!class /Script/Engine.Controller))) (Variables|Default|GetInitialPitch) _alpha) (.Yaw (Math|Rotator|BreakRotator (Pawn|GetControlRotation _myplayercontroller :!class /Script/Engine.Controller)))))
                    (else
                      (Pawn|SetControlRotation _myplayercontroller (Math|Rotator|MakeRotator (.Roll (Math|Rotator|BreakRotator (Pawn|GetControlRotation _myplayercontroller :!class /Script/Engine.Controller))) (Math|Float|Lerp (- (.Pitch (Math|Rotator|BreakRotator (Pawn|GetControlRotation _myplayercontroller :!class /Script/Engine.Controller))) 3.6e+02) (Variables|Default|GetInitialPitch) _alpha) (.Yaw (Math|Rotator|BreakRotator (Pawn|GetControlRotation _myplayercontroller :!class /Script/Engine.Controller)))))))
                  (bind _myplayercontroller_2 (CallFunction|GetMyPlayerController))
                  (if (<= (Math|Float|Absolute(Float) (- (.Pitch (Math|Rotator|BreakRotator (Pawn|GetControlRotation _myplayercontroller_2 :!class /Script/Engine.Controller))) (Variables|Default|GetInitialPitch))) 0.5)
                    (Variables|Default|SetInitialPitch 0.0)
                    (Timeline|StopRecoilTimeLine Stop)))))))))))

(event EventUpdateAmmoHUD
  ;[1 0.3487 0.2889] UpdateAmmo
  (Utilities|FlowControl|Delay 0.05)
  (bind _aspawn (Utilities|Casting|CastToPawn (Components|GetOwner)))
  (bind _asplayer_controller (Utilities|Casting|CastToPlayerController (Pawn|GetController _aspawn)))
  (bind _asbp_mbfpsmain_hud (Utilities|Casting|CastToBP_MBFPSMainHUD (HUD|GetHUD _asplayer_controller)))
  (bind _returnvalue (Class|Weapon|GetMaxAmmo))
  (bind _returnvalue_2 (Class|Weapon|GetCurrentAmmo))
  (Default|UpdateAmmoHUD (Variables|/Game/Blueprints/HUD/BP_MBFPSMainHUD.BP_MBFPSMainHUD_C|GetMainHUD _asbp_mbfpsmain_hud) _returnvalue_2 _returnvalue (Variables|Default|GetWeaponIcon)))

(fn ConstructionScript)

(fn ApplyRecoil
  (params (PitchInput :type Float%20%28single-precision%29) (yawInput :type Float%20%28single-precision%29))
  (bind _myplayercontroller (CallFunction|GetMyPlayerController))
  (Class|PlayerController|AddPitchInput _myplayercontroller (* PitchInput -1.0))
  (Class|PlayerController|AddYawInput _myplayercontroller yawInput))

(fn GetMyPlayerController
  (bind _aspawn (Utilities|Casting|CastToPawn (Components|GetOwner)))
  (bind _asplayer_controller (Utilities|Casting|CastToPlayerController (Pawn|GetController _aspawn)))
  (return _asplayer_controller))